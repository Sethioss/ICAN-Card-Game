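; Player state for a card game that spawns and manages the player's hand of cards.
; BeginPlay spawns the configured hand collection at its class-default origin transform and caches its capacity.
; OWN-prefixed events insert or remove card IDs by index and rebuild the hand visuals, with removal also deselecting every card.
; It also records the selected card's index and ID (-1 if none), reports whether the hand is full, and offers debug printing.
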(event `self.ReceiveBeginPlay`
  (bind _handcollectiontouse (`self.HandCollectionToUse`))
  (bind (_origintransform _maxcapacity) (defaults `Object` _handcollectiontouse))
  (set `self.HandSize` _maxcapacity)
  (bind _returnvalue (`|SpawnActorFromClass` _handcollectiontouse _origintransform "Undefined" "MultiplyWithRoot" null null))
  (set `self.Hand` _returnvalue))

(event `DebugHand`
  ;[1 0.7919 0.3931] Hand
  ;;[1 1 1] Debug Cards
  (for _array_element (`CardCollection.Cards` (`self.Hand`))
    (`KismetSystemLibrary.PrintString` (`KismetStringLibrary.Concat_StrStr` (`CardData.Name` (`Card.CardDataComp` _array_element)) (`KismetStringLibrary.Conv_BoolToString` (`Card.bIsCardSelected` _array_element))) true true (struct :`R` 1.0 :`G` 0.670951 :`A` 1.0) 999.0))
  (`KismetSystemLibrary.PrintString` "Hand----------------------------" true true (struct :`R` 1.0 :`G` 0.534703 :`A` 1.0) 99.0))

(event `OWN-AddCardToHand`
  (params (ID :type Integer) (Location :type Integer))
  (bind _hand (`self.Hand`))
  ;[1 0.7919 0.3931] Hand
  (`KismetArrayLibrary.Array_Insert` (`CardCollection.Contents` _hand) ID Location)
  (bind _asbp_hand (cast `/Game/Blueprint/BP_Hand` _hand))
  (`/Game/Blueprint/BP_Hand.InitializeHandVisuals` _asbp_hand))

(event `OWN-RemoveHandCardAtLocation`
  (params (Location :type Integer))
  (bind _hand (`self.Hand`))
  ;[1 0.7919 0.3931] Hand
  (`KismetArrayLibrary.Array_Remove` (`CardCollection.Contents` _hand) Location)
  (for _array_element (`CardCollection.Cards` _hand)
    (bind _asbp_standard_card (cast `/Game/Blueprint/Cards/BP_StandardCard` _array_element))
    (`/Game/Blueprint/Cards/BP_StandardCard.OWN-DeselectCard` _asbp_standard_card))
  (bind _asbp_hand (cast `/Game/Blueprint/BP_Hand` _hand))
  (`/Game/Blueprint/BP_Hand.InitializeHandVisuals` _asbp_hand))

(event `OWN-GetSelectedCard`
  (set `self.SelectedCardInHandLocation` -1)
  (set `self.SelectedCardInHandID` -1)
  (for (_array_element _array_index) (`CardCollection.Cards` (`self.Hand`))
    (bind _asbp_standard_card (cast `/Game/Blueprint/Cards/BP_StandardCard` _array_element))
    (if (`Card.bIsCardSelected` _asbp_standard_card)
      (set `self.SelectedCardInHandLocation` _array_index)
      (set `self.SelectedCardInHandID` (`Card.CardID` _asbp_standard_card)))))

(fn `IsHandFull`
  (returns (IsFull :type Boolean))
  (bind _hand (`self.Hand`))
  (return (>= (`KismetArrayLibrary.Array_Length` (`CardCollection.Contents` _hand)) (`CardCollection.MaxCapacity` _hand))))

(fn `UserConstructionScript`)