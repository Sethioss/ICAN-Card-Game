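; Server game mode for a multiplayer co-op card game where the team fights random data-table enemies.
; Drives BP_SM_MainStateMachine from lobby through timed rounds to win or fail, exposing events for each phase.
; Rounds refill hands, open a countdown play phase, then compare the played mat's score to enemy health, costing team health on failure.
; Pushes UI and input to BP_CardControllers via owner events; multicast events handle card actors.
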(event `SRV-SpawnCountdownWidget`
  (params (`Card Controller` :type "/Game/Blueprint/Controller/BP_CardController Object Reference"))
  ;[1 0.8232 0.1521] Widgets Handling
  (bind _output_get (set `self.PlayablePhaseCurrentTime` (`self.PlayablePhaseDuration`)))
  (`/Game/Blueprint/Controller/BP_CardController.OWN-SpawnCountdownWidget` `Card Controller` _output_get))

(event `SRV-UpdateCountdown`
  ;[1 0.8232 0.1521] Widgets Handling
  (bind _output_get (set `self.PlayablePhaseCurrentTime` (- (`self.PlayablePhaseCurrentTime`) (`GameplayStatics.GetWorldDeltaSeconds`))))
  (for _array_element (`GameStateBase.PlayerArray` (`GameplayStatics.GetGameState`))
    (bind _asbp_card_controller (cast `/Game/Blueprint/Controller/BP_CardController` (`PlayerState.GetPlayerController` _array_element)))
    (`/Game/Blueprint/Controller/BP_CardController.OWN-UpdateCountdownWidget` _asbp_card_controller (`KismetMathLibrary.FMax` _output_get)))
  (if (not (> _output_get 0.0))
    (bind _asbp_sm_main_state_machine (cast `/Game/Blueprint/StateSystem/BP_SM_MainStateMachine` (`self.StateMachine`)))
    (`/Game/Blueprint/StateSystem/BP_SM_MainStateMachine.SRV-ChangeStateTo` _asbp_sm_main_state_machine "Resolve" true _asbp_sm_main_state_machine)))

(event `MTC-ClearPlayedCardActorList`
  (params (PlayedCard :type "PlayedCardMat Object Reference"))
  (bind _cards (`CardCollection.Cards` PlayedCard))
  ;[1 1 1] Misc/Uitlitaries
  (for _array_element _cards
    (`/Engine/EditorBlueprintResources/StandardMacros.IsValid` _array_element
      (:`Is Valid`
        (`self.K2_DestroyActor` _array_element))))
  (`KismetArrayLibrary.Array_Clear` _cards)
  (`KismetArrayLibrary.Array_Resize` _cards 3))

(event `self.ReceiveBeginPlay`
  (set `self.TeamHealth` (`self.TeamMaxHealth`))
  (bind _returnvalue (`GameplayStatics.GetActorOfClass` "/Game/Blueprint/StateSystem/BP_SM_MainStateMachine.BP_SM_MainStateMachine_C"))
  (set `self.StateMachine` _returnvalue)
  (`self.SRV-InitFSM`))

(event `SRV-DebugCardActorLength`
  (params (Cards :type "Array of Card Object Reference"))
  ;[1 1 1] Misc/Uitlitaries
  (`KismetSystemLibrary.PrintString` (`KismetStringLibrary.Conv_IntToString` (`KismetArrayLibrary.Array_Length` Cards)) true true (struct :`R` 1.0 :`B` 0.930323 :`A` 1.0) 10.0))

(event `SRV-RemoveMainUI`
  (params (CardController :type "/Game/Blueprint/Controller/BP_CardController Object Reference"))
  ;[1 0.8232 0.1521] Widgets Handling
  (`/Game/Blueprint/Controller/BP_CardController.OWN-RemoveWidgets` CardController))

(event `SRV-InitFSM`
  (bind _asbp_sm_main_state_machine (cast `/Game/Blueprint/StateSystem/BP_SM_MainStateMachine` (`self.StateMachine`)))
  (`/Game/Blueprint/StateSystem/BP_SM_MainStateMachine.SRV-ChangeStateTo` _asbp_sm_main_state_machine "Test" false _asbp_sm_main_state_machine))

(event `SRV-SpawnMainUI`
  (params (CardController :type "/Game/Blueprint/Controller/BP_CardController Object Reference"))
  ;[1 0.8232 0.1521] Widgets Handling
  (`/Game/Blueprint/Controller/BP_CardController.OWN-SpawnHostUI` CardController (`GameplayStatics.GetObjectClass` (`self.HostUI`)) (`self.MaxPlayerNumber`) (`KismetArrayLibrary.Array_Length` (`self.PlayerList`))))

(event `MTC-SetCardData`
  (params (Card :type "Card Object Reference") (CardID :type Integer))
  (bind _carddatacomp (`Card.CardDataComp` Card))
  ;[1 1 1] Misc/Uitlitaries
  (bind _returnvalue (`|GetDataTableRow` (`self.DeckDataTable`) (`KismetStringLibrary.Conv_StringToName` (`KismetStringLibrary.Conv_IntToString` CardID)))
    (:`then`
      (bind (_name _strength _placement _cardmat _elementmat) (break `/Game/Tables/S_CardStruct` _returnvalue))
      (set `CardData.Name` (`KismetTextLibrary.Conv_TextToString` _name) _carddatacomp)
      (set `CardData.Strength` _strength _carddatacomp)
      (set `CardData.Placement` _placement _carddatacomp)
      (bind _asbp_standard_card (cast `/Game/Blueprint/Cards/BP_StandardCard` Card))
      (`/Game/Blueprint/Cards/BP_StandardCard.SetCardText` _asbp_standard_card _asbp_standard_card)
      (set `/Game/Blueprint/Cards/BP_StandardCard.CardBodyMat` _cardmat _asbp_standard_card)
      (set `/Game/Blueprint/Cards/BP_StandardCard.CardElementMat` _elementmat _asbp_standard_card))))

(event `self.K2_PostLogin`
  (params (NewPlayer :type "PlayerController Object Reference"))
  (`KismetArrayLibrary.Array_AddUnique` (`self.PlayerList`) NewPlayer)
  (for _array_element (`GameStateBase.PlayerArray` (`GameplayStatics.GetGameState`))
    (bind _asbp_card_controller (cast `/Game/Blueprint/Controller/BP_CardController` (`PlayerState.GetPlayerController` _array_element)))
    (`self.SRV-RemoveMainUI` _asbp_card_controller)
    (`self.SRV-SpawnMainUI` _asbp_card_controller))
  (if (>= (`KismetArrayLibrary.Array_Length` (`GameStateBase.PlayerArray` (`GameplayStatics.GetGameState`))) (`self.MaxPlayerNumber`))
    (bind _asbp_sm_main_state_machine (cast `/Game/Blueprint/StateSystem/BP_SM_MainStateMachine` (`self.StateMachine`)))
    (`/Game/Blueprint/StateSystem/BP_SM_MainStateMachine.SRV-ChangeStateTo` _asbp_sm_main_state_machine "Warmup" true _asbp_sm_main_state_machine)))

(event `SRV-SpawnGameOverUI`
  (params (`Card Controller` :type "/Game/Blueprint/Controller/BP_CardController Object Reference"))
  ;[1 0.8232 0.1521] Widgets Handling
  (`/Game/Blueprint/Controller/BP_CardController.OWN-SpawnGameOverUI` `Card Controller`))

(event `SRV-ClearDeckCardActorList`
  (params (Deck :type "Deck Object Reference"))
  (bind _cards (`CardCollection.Cards` Deck))
  ;[1 1 1] Misc/Uitlitaries
  (for _array_element _cards
    (`self.K2_DestroyActor` _array_element))
  (`KismetArrayLibrary.Array_Clear` _cards))

(event `SRV-SpawnWinUI`
  (params (`Card Controller` :type "/Game/Blueprint/Controller/BP_CardController Object Reference"))
  ;[1 0.8232 0.1521] Widgets Handling
  (`/Game/Blueprint/Controller/BP_CardController.OWN-SpawnWinUI` `Card Controller`))

(event `MTC-SpawnNewCardInPlayedSlots`
  (params (Transform :type "Transform Structure") (PlayedCardMat :type "PlayedCardMat Object Reference") (CardID :type Integer) (CardLocation :type Integer))
  ;[0 0.6208 1] PlayedCardSlots
  (`self.MTC-SpawnCardInPlayedMat` Transform PlayedCardMat CardID CardLocation))

(event `SRV-StartWarmUp`
  (bind _warmupduration (`self.WarmUpDuration`))
  (`KismetSystemLibrary.PrintString` (`KismetStringLibrary.Concat_StrStr` (`KismetStringLibrary.Concat_StrStr` "All players have logged in! Starting game in " (`KismetStringLibrary.Conv_DoubleToString` _warmupduration)) " seconds...") true true (struct :`G` 0.66 :`B` 1.0 :`A` 1.0) 5.0)
  (`KismetSystemLibrary.Delay` _warmupduration)
  (bind _asbp_sm_main_state_machine (cast `/Game/Blueprint/StateSystem/BP_SM_MainStateMachine` (`self.StateMachine`)))
  (`/Game/Blueprint/StateSystem/BP_SM_MainStateMachine.SRV-ChangeStateTo` _asbp_sm_main_state_machine "Start" false _asbp_sm_main_state_machine))

(event `SRV-DebugPlayedCards`
  ;[0 0.6208 1] PlayedCardSlots
  (for _array_element (`CardCollection.Contents` (`self.PlayedCards`))
    (`KismetSystemLibrary.PrintString` (`KismetStringLibrary.Conv_IntToString` _array_element) true true (struct :`G` 0.66 :`B` 1.0 :`A` 1.0) 10.0)))

(event `SRV-BeginGame`
  ;[1 1 1] Game Start
  (for _array_element (`GameStateBase.PlayerArray` (`GameplayStatics.GetGameState`))
    (bind _asbp_card_controller (cast `/Game/Blueprint/Controller/BP_CardController` (`PlayerState.GetPlayerController` _array_element)))
    (`self.SRV-RemoveMainUI` _asbp_card_controller))
  (`self.SRV-CreatePlayingField`)
  (`self.SRV-StartNewRound`))

(event `SRV-SetPlayedCard`
  (params (IDToAdd :type Integer) (Location :type Integer))
  (bind _playedcards (`self.PlayedCards`))
  ;[0 0.6208 1] PlayedCardSlots
  (`KismetArrayLibrary.Array_Set` (`CardCollection.Contents` _playedcards) Location IDToAdd)
  (bind _asbp_played_card_mat (cast `/Game/Blueprint/BP_PlayedCardMat` _playedcards))
  (`/Game/Blueprint/BP_PlayedCardMat.SRV-UpdateCollectionContent` _asbp_played_card_mat _playedcards)
  (`/Game/Blueprint/BP_PlayedCardMat.OWN-CheckIfMatFull` _asbp_played_card_mat))

(event `SRV-StartNewRound`
  (bind _playedcards (`self.PlayedCards`))
  (`KismetSystemLibrary.Delay` (`self.NewRoundWarmupDuration`))
  (bind _asbp_played_card_mat (cast `/Game/Blueprint/BP_PlayedCardMat` _playedcards))
  (`/Game/Blueprint/BP_PlayedCardMat.MTC-EmptyCardMat` _asbp_played_card_mat _asbp_played_card_mat)
  (`/Game/Blueprint/BP_PlayedCardMat.SRV-UpdateCollectionContent` _asbp_played_card_mat _playedcards)
  (for _array_element (`GameStateBase.PlayerArray` (`GameplayStatics.GetGameState`))
    (bind _asbp_player_state (cast `/Game/Blueprint/Online/BP_PlayerState` _array_element))
    (bind _asbp_card_controller (cast `/Game/Blueprint/Controller/BP_CardController` (`PlayerState.GetPlayerController` _asbp_player_state)))
    (`self.SRV-FillHand` _asbp_card_controller (`self.DeckDataTable`)))
  (bind _asbp_played_card_mat_2 (cast `/Game/Blueprint/BP_PlayedCardMat` (`self.PlayedCards`)))
  (`/Game/Blueprint/BP_ScoreCalculator.SRV-ResetCalc` (`/Game/Blueprint/BP_PlayedCardMat.ScoreCalc` _asbp_played_card_mat_2))
  (bind _asbp_sm_main_state_machine (cast `/Game/Blueprint/StateSystem/BP_SM_MainStateMachine` (`self.StateMachine`)))
  (`/Game/Blueprint/StateSystem/BP_SM_MainStateMachine.SRV-ChangeStateTo` _asbp_sm_main_state_machine "EnemySpawn" true _asbp_sm_main_state_machine)
  (`KismetSystemLibrary.PrintString` "New round will start soon" true true (struct :`R` 1.0 :`B` 0.962626 :`A` 1.0))
  (`KismetSystemLibrary.Delay` (`self.EnemyToPlayDuration`))
  (`/Game/Blueprint/StateSystem/BP_SM_MainStateMachine.SRV-ChangeStateTo` _asbp_sm_main_state_machine "PlayPhase" true _asbp_sm_main_state_machine))

(event `MTC-InitPlayedMat`
  (params (PlayedCards :type "PlayedCardMat Object Reference"))
  ;[0 0.6208 1] PlayedCardSlots
  (bind _output_get (set `self.CardSlotArray` (`self.K2_GetComponentsByClass` PlayedCards "/Script/ICAN_Card_Game.CardSlotComponent")))
  (set `CardCollection.MaxCapacity` (`KismetArrayLibrary.Array_Length` _output_get) PlayedCards))

(event `SRV-CreatePlayingField`
  (bind _playedcardscollectiontouse (`self.PlayedCardsCollectionToUse`))
  ;[0 0.6208 1] PlayedCardSlots
  (bind _returnvalue (`|SpawnActorFromClass` _playedcardscollectiontouse (`.OriginTransform` (defaults `Object` _playedcardscollectiontouse)) "Undefined" "MultiplyWithRoot" null null))
  (bind _output_get (set `self.PlayedCards` _returnvalue))
  (`self.MTC-InitPlayedMat` _output_get))

(event `SRV-FillHand`
  (params (Controller :type "/Game/Blueprint/Controller/BP_CardController Object Reference") (`Data Table` :type "DataTable Object Reference"))
  (`/Game/Blueprint/Controller/BP_CardController.OWN-FillHand` Controller `Data Table`))

(event `MTC-SpawnCardInPlayedMat`
  (params (Transform :type "Transform Structure") (PlayedCardMat :type "PlayedCardMat Object Reference") (CardID :type Integer) (CardLocation :type Integer))
  ;[0 0.6208 1] PlayedCardSlots
  (bind _returnvalue (`|SpawnActorFromClass` "/Game/Blueprint/Cards/BP_StandardCard.BP_StandardCard_C" Transform "Undefined" "MultiplyWithRoot" null null))
  (set `Card.Status` "IN_SLOT" _returnvalue)
  (bind _output_get (set `Card.CardID` CardID _returnvalue))
  (`KismetArrayLibrary.Array_Set` (`CardCollection.Cards` PlayedCardMat) CardLocation _returnvalue)
  (`self.MTC-SetCardData` _returnvalue _output_get))

(event `SRV-SpawnEnemy`
  (bind _enemytable (`self.EnemyTable`))
  (bind _outrownames (`DataTableFunctionLibrary.GetDataTableRowNames` _enemytable))
  (bind _returnvalue (`|GetDataTableRow` _enemytable (`KismetArrayLibrary.Array_Random` _outrownames))
    (:`then`
      (bind _enemybp (break `/Game/Tables/S_EnemyStruct` _returnvalue))
      (bind _returnvalue_2 (`|SpawnActorFromClass` _enemybp (`KismetMathLibrary.MakeTransform` (110.0 230.0 0.0) (`.SpawnRotation` (defaults `Object` _enemybp))) "Undefined" "MultiplyWithRoot" null null))
      (set `self.CurrentEnemy` _returnvalue_2))))

(event `SRV-StartPlayablePhase`
  (for _array_element (`GameStateBase.PlayerArray` (`GameplayStatics.GetGameState`))
    (bind _asbp_card_controller (cast `/Game/Blueprint/Controller/BP_CardController` (`PlayerState.GetPlayerController` _array_element)))
    (`/Game/Blueprint/Controller/BP_CardController.OWN-SetPlayable` _asbp_card_controller true)
    (`self.SRV-SpawnCountdownWidget` _asbp_card_controller)))

(event `SRV-StartResolvePhase`
  (bind _currentenemy (`self.CurrentEnemy`))
  (for _array_element (`GameStateBase.PlayerArray` (`GameplayStatics.GetGameState`))
    (bind _asbp_card_controller (cast `/Game/Blueprint/Controller/BP_CardController` (`PlayerState.GetPlayerController` _array_element)))
    (`/Game/Blueprint/Controller/BP_CardController.OWN-SetPlayable` _asbp_card_controller false))
  (bind _asbp_played_card_mat (cast `/Game/Blueprint/BP_PlayedCardMat` (`self.PlayedCards`)))
  (bind _scorecalc (`/Game/Blueprint/BP_PlayedCardMat.ScoreCalc` _asbp_played_card_mat))
  (if (not (`/Game/Blueprint/BP_ScoreCalculator.IsFull` _scorecalc))
    (`/Game/Blueprint/BP_PlayedCardMat.SRV-CalculateScore` _asbp_played_card_mat _scorecalc))
  (set `/Game/Blueprint/BP_ScoreCalculator.IsFull` false _scorecalc)
  (if (> (`/Game/Blueprint/BP_ScoreCalculator.FinalResult` _scorecalc) (`Enemy.Health` (`self.CurrentEnemy`)))
    (`KismetSystemLibrary.PrintString` "You killed the enemy!!!" true true (struct :`R` 0.055069 :`G` 1.0 :`A` 1.0) 5.0)
    (`self.K2_DestroyActor` (`self.CurrentEnemy`))
    (set `self.EnemiesRemaining` (- (`self.EnemiesRemaining`) 1))
    (if (<= (`self.EnemiesRemaining`) 0)
      (`KismetSystemLibrary.PrintString` "You win!!!" true true (struct :`R` 0.051391 :`G` 1.0 :`A` 1.0))
      (bind _asbp_sm_main_state_machine (cast `/Game/Blueprint/StateSystem/BP_SM_MainStateMachine` (`self.StateMachine`)))
      (`/Game/Blueprint/StateSystem/BP_SM_MainStateMachine.SRV-ChangeStateTo` _asbp_sm_main_state_machine "Win" true _asbp_sm_main_state_machine)
      (else
        (if (> (stale _output_get) 0) :!label _label
          (`/Engine/EditorBlueprintResources/StandardMacros.IsValid` _currentenemy
            (:`Is Valid`
              (`self.K2_DestroyActor` _currentenemy))
            (:`Is Not Valid`
              _))
          (`self.SRV-StartNewRound`)
          (else
            (bind _asbp_sm_main_state_machine_2 (cast `/Game/Blueprint/StateSystem/BP_SM_MainStateMachine` (`self.StateMachine`)))
            (`/Game/Blueprint/StateSystem/BP_SM_MainStateMachine.SRV-ChangeStateTo` _asbp_sm_main_state_machine_2 "Fail" true _asbp_sm_main_state_machine_2)))))
    (else
      (`KismetSystemLibrary.PrintString` "You didn't do shit :'(" true true (struct :`R` 1.0 :`G` 0.16801 :`A` 1.0) 5.0)
      (bind _output_get (set `self.TeamHealth` (- (`self.TeamHealth`) 1)))
      (`KismetSystemLibrary.PrintString` (`KismetStringLibrary.Concat_StrStr` "New health: " (`KismetStringLibrary.Conv_IntToString` _output_get)))
      (goto _label))))

(event `SRV-ShowGameOver`
  (for _array_element (`GameStateBase.PlayerArray` (`GameplayStatics.GetGameState`))
    (bind _asbp_card_controller (cast `/Game/Blueprint/Controller/BP_CardController` (`PlayerState.GetPlayerController` _array_element)))
    (`self.SRV-SpawnGameOverUI` _asbp_card_controller)))

(event `SRV-ShowWin`
  (for _array_element (`GameStateBase.PlayerArray` (`GameplayStatics.GetGameState`))
    (bind _asbp_card_controller (cast `/Game/Blueprint/Controller/BP_CardController` (`PlayerState.GetPlayerController` _array_element)))
    (`self.SRV-SpawnWinUI` _asbp_card_controller)))

(fn `IsDeckEmpty`
  (returns (IsEmpty :type Boolean))
  (return (<= (`KismetArrayLibrary.Array_Length` (`CardCollection.Contents` (`self.Deck`))) 0)))

(fn `SRV_FillDeck`)

(fn `UserConstructionScript`)