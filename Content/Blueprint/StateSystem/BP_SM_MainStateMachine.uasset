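; Main state machine Blueprint that switches the current state by name, with each state represented by an actor class.
; SRV-ChangeStateTo skips a valid same-named state, otherwise matches States by class-default Name and reuses that actor from the world or spawns one.
; It then activates its own CurrentState and calls StartDelegate.
; The previous state is deactivated only when an existing actor is reused, and PlaysTransition is unused.
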(event `SRV-ChangeStateTo`
  (params (StateName :type String) (PlaysTransition :type Boolean) (StateMachine :type "/Game/Blueprint/StateSystem/BP_SM_MainStateMachine Object Reference"))
  (bind _currentstate (`CardGameFSM.CurrentState` StateMachine))
  (bind _currentstate_2 (`self.CurrentState`))
  (`/Engine/EditorBlueprintResources/StandardMacros.IsValid` _currentstate
    (:`Is Valid`
      (if (not (== (`CardFSMState.Name` _currentstate) StateName))
        (for _array_element (`self.States`) :!label _label
          (if (== StateName (defaults `Object` _array_element))
            (bind _returnvalue (`GameplayStatics.GetActorOfClass` _array_element))
            (`/Engine/EditorBlueprintResources/StandardMacros.IsValid` _returnvalue
              (:`Is Valid`
                (set `CardFSMState.bActiveState` false _currentstate)
                (set `CardGameFSM.CurrentState` _returnvalue StateMachine))
              (:`Is Not Valid`
                (bind _returnvalue_2 (`|SpawnActorFromClass` _array_element (`KismetMathLibrary.MakeTransform` (0.0 0.0 0.0)) "Undefined" "MultiplyWithRoot" null null))
                (set `CardFSMState.bActiveState` false _returnvalue_2)
                (set `CardGameFSM.CurrentState` _returnvalue_2 StateMachine)))
            (`KismetSystemLibrary.PrintString` "Successfully changed state!")))
        (set `CardFSMState.bActiveState` true _currentstate_2)
        (`CardFSMState.StartDelegate` _currentstate_2)))
    (:`Is Not Valid`
      (goto _label))))

(fn `UserConstructionScript`)