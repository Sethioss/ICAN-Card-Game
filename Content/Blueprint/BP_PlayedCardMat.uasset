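; BP_PlayedCardMat is the mat for played cards, tracking card IDs per slot, the card actors and whether it is full.
; On content updates, it has BP_CardGameMode clear the old card actors, plays a sound and respawns non-negative IDs at slot locations.
; Emptying sets slots to -1, while a separate function destroys card actors.
; BP_ScoreCalculator receives the full flag and scores the cards, though one scoring call is unwired.
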(event `self.ReceiveBeginPlay`
  (bind _returnvalue (`GameplayStatics.GetActorOfClass` "/Game/Blueprint/BP_ScoreCalculator.BP_ScoreCalculator_C"))
  (set `self.ScoreCalc` _returnvalue)
  (bind _returnvalue_2 (`GameplayStatics.GetActorOfClass` "/Script/Engine.TextRenderActor"))
  (bind _output_get (set `ScoreCalculator.TextActor` _returnvalue_2 (`/Game/Blueprint/BP_ScoreCalculator.ScoreCalculator` (`self.ScoreCalc`))))
  (`TextRenderComponent.K2_SetText` (`TextRenderActor.TextRender` _output_get) "Hello!"))

(event `OWN-CheckIfMatFull`
  (if (>= (`KismetArrayLibrary.Array_Length` (`self.Cards`)) (`self.MaxCapacity`))
    (set `/Game/Blueprint/BP_ScoreCalculator.IsFull` true (`self.ScoreCalc`))))

(event `MTC-EmptyCardMat`
  (params (`Card Mat` :type "PlayedCardMat Object Reference"))
  (bind _contents (`CardCollection.Contents` `Card Mat`))
  (for (_ _array_index) _contents
    (`KismetArrayLibrary.Array_Set` _contents _array_index -1)))

(event `SRV-CalculateScore`
  (params (ScoreCalc :type "/Game/Blueprint/BP_ScoreCalculator Object Reference"))
  (bind _returnvalue (`ScoreCalculator.CalculateScore` (`/Game/Blueprint/BP_ScoreCalculator.ScoreCalculator` ScoreCalc) (`self.Cards`)))
  (set `/Game/Blueprint/BP_ScoreCalculator.FinalResult` _returnvalue ScoreCalc))

(event `SRV-UpdateCollectionContent`
  (params (CardMat :type "PlayedCardMat Object Reference"))
  (bind _contents (`CardCollection.Contents` CardMat))
  (bind _asbp_card_game_mode (cast `/Game/Blueprint/Online/BP_CardGameMode` (`GameplayStatics.GetGameMode`)))
  (`/Game/Blueprint/Online/BP_CardGameMode.MTC-ClearPlayedCardActorList` _asbp_card_game_mode CardMat)
  (`GameplayStatics.PlaySound2D` "/Game/Sounds/SFX/S_CardPlayed_Cue.S_CardPlayed_Cue" 1.0 1.0 0.0 null null)
  (for (_array_element _array_index) _contents
    (if (`KismetArrayLibrary.Array_IsValidIndex` _contents _array_index)
      (bind _asbp_card_game_mode_2 (cast `/Game/Blueprint/Online/BP_CardGameMode` (`GameplayStatics.GetGameMode`)))
      (if (>= _array_element 0)
        (`/Game/Blueprint/Online/BP_CardGameMode.MTC-SpawnNewCardInPlayedSlots` _asbp_card_game_mode (`KismetMathLibrary.MakeTransform` (`SceneComponent.K2_GetComponentLocation` (`|GetArrayItem` (`/Game/Blueprint/Online/BP_CardGameMode.CardSlotArray` _asbp_card_game_mode_2) _array_index)) (struct :`Pitch` -90.0)) CardMat _array_element _array_index)))))

(fn `EmptyCards`
  (bind _cards (`self.Cards`))
  (for _array_element _cards
    (`/Engine/EditorBlueprintResources/StandardMacros.IsValid` _array_element
      (:`Is Valid`
        (`self.K2_DestroyActor` _array_element))))
  (`KismetArrayLibrary.Array_Clear` _cards))

(fn `UserConstructionScript`)