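; Player-side Blueprint for a card game that turns mouse clicks into hand selection and card placement on the play mat.
; When the controller allows play, cursor line traces on two channels find either a hand card to toggle, with single selection, or a mat slot.
; Slot clicks go through SRV/OWN-prefixed events that check the game mode's played cards, then place the selected card or swap it with the occupant, updating the player state's hand.
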(event `self.OnClickBP`
  (`self.OWN-Handle click`))

(event `OWN-Handle click`
  (bind _returnvalue (`self.GetController`))
  (bind _asbp_card_controller (cast `/Game/Blueprint/Controller/BP_CardController` _returnvalue)
    (:`then`
      (if (`/Game/Blueprint/Controller/BP_CardController.bCanPlay` _asbp_card_controller)
        (bind _ascard_player_controller (cast `CardPlayerController` _returnvalue))
        (bind (_locationx _locationy) (`PlayerController.GetMousePosition` _ascard_player_controller))
        (bind (_worldposition _worlddirection) (`GameplayStatics.DeprojectScreenToWorld` _ascard_player_controller (`KismetMathLibrary.MakeVector2D` _locationx _locationy)))
        (bind _returnvalue_2 (* _worlddirection 5000))
        ;[1 1 1] If card hit
        (bind _outhit (`KismetSystemLibrary.LineTraceSingle` _worldposition _returnvalue_2 "TraceTypeQuery4"))
        (bind (_bblockinghit _binitialoverlap _time _distance _location _impactpoint _normal _impactnormal _physmat _hitactor) (`GameplayStatics.BreakHitResult` _outhit))
        (if _bblockinghit
          (bind _ascard (cast `Card` _hitactor))
          (`/Engine/EditorBlueprintResources/StandardMacros.IsValid` _ascard
            (:`Is Valid`
              (if (`|EnumEquality` (`Card.Status` _ascard) "IN_HAND")
                (if (!= true (`Card.bIsCardSelected` _ascard))
                  (bind _ascgplayer_state (cast `CGPlayerState` (`GameplayStatics.GetPlayerState` 0)))
                  (for _array_element (`CardCollection.Cards` (`CGPlayerState.Hand` _ascgplayer_state))
                    (bind _asbp_standard_card (cast `/Game/Blueprint/Cards/BP_StandardCard` _array_element))
                    (`self.OWN-Deselect Card` _asbp_standard_card))
                  (bind _asbp_standard_card_2 (cast `/Game/Blueprint/Cards/BP_StandardCard` _ascard))
                  (`self.OWN-Select Card` _asbp_standard_card_2)
                  (else
                    (bind _asbp_standard_card_3 (cast `/Game/Blueprint/Cards/BP_StandardCard` _ascard))
                    (`/Game/Blueprint/Cards/BP_StandardCard.OWN-DeselectCard` _asbp_standard_card_3)))
                (bind _asbp_player_state (cast `/Game/Blueprint/Online/BP_PlayerState` _ascgplayer_state))
                (else
                  ;[1 1 1] If PlayedMat Slot hit
                  (bind _outhit_2 (`KismetSystemLibrary.LineTraceSingle` _worldposition _returnvalue_2 "TraceTypeQuery6" :!label _label))
                  (bind (_bblockinghit_2 _binitialoverlap_2 _time_2 _distance_2 _location_2 _impactpoint_2 _normal_2 _impactnormal_2 _physmat_2 _hitactor_2 _hitcomponent) (`GameplayStatics.BreakHitResult` _outhit_2))
                  (if _bblockinghit_2
                    (bind _ascard_slot_component (cast `CardSlotComponent` _hitcomponent))
                    (`self.SRV-HandleClickOnMatCard` _ascard_slot_component))))))
          (else
            (goto _label)))))
    (:`CastFailed`
      (`KismetSystemLibrary.PrintString` "Couldn't get controller"))))

(event `OWN-Select Card`
  (params (Card :type "/Game/Blueprint/Cards/BP_StandardCard Object Reference"))
  ;[1 1 1] If card hit
  (`/Game/Blueprint/Cards/BP_StandardCard.OWN-SelectCard` Card))

(event `OWN-Deselect Card`
  (params (Card :type "/Game/Blueprint/Cards/BP_StandardCard Object Reference"))
  ;[1 1 1] If card hit
  (`/Game/Blueprint/Cards/BP_StandardCard.OWN-DeselectCard` Card))

(event `SRV-Set Played Card`
  (params (CardID :type Integer) (Location :type Integer))
  ;[1 1 1] Add card to played slot
  (bind _asbp_card_game_mode (cast `/Game/Blueprint/Online/BP_CardGameMode` (`GameplayStatics.GetGameMode`)))
  (`/Game/Blueprint/Online/BP_CardGameMode.SRV-SetPlayedCard` _asbp_card_game_mode CardID Location))

(event `OWN-AddCardToPlayedSlot`
  (`|ExecutionSequence`
    (:`then_0`
      ;[1 1 1] Add card to played slot
      (bind _asbp_player_state (cast `/Game/Blueprint/Online/BP_PlayerState` (`GameplayStatics.GetPlayerState` 0)))
      (`/Game/Blueprint/Online/BP_PlayerState.OWN-GetSelectedCard` _asbp_player_state)
      (bind _selectedcardinhandid (`/Game/Blueprint/Online/BP_PlayerState.SelectedCardInHandID` _asbp_player_state))
      (if (>= _selectedcardinhandid 0)
        (`self.SRV-Set Played Card` _selectedcardinhandid (`CardSlotComponent.ID` (stale `OWN-Handle click` _ascard_slot_component)))))
    (:`then_1`
      ;[1 1 1] Remove card from hand
      (`self.OWN-RemoveSelectedCardFromHand`))))

(event `OWN-RemoveSelectedCardFromHand`
  ;[1 1 1] Remove card from hand
  (bind _asbp_player_state (cast `/Game/Blueprint/Online/BP_PlayerState` (`GameplayStatics.GetPlayerState` 0)))
  (`/Game/Blueprint/Online/BP_PlayerState.OWN-GetSelectedCard` _asbp_player_state)
  (bind _selectedcardinhandlocation (`/Game/Blueprint/Online/BP_PlayerState.SelectedCardInHandLocation` _asbp_player_state))
  (if (>= _selectedcardinhandlocation 0)
    (`/Game/Blueprint/Online/BP_PlayerState.OWN-RemoveHandCardAtLocation` _asbp_player_state _selectedcardinhandlocation)))

(event `SRV-HandleClickOnMatCard`
  (params (CardSlotComp :type "CardSlotComponent Object Reference"))
  (bind _id (`CardSlotComponent.ID` CardSlotComp))
  (bind _asbp_card_game_mode (cast `/Game/Blueprint/Online/BP_CardGameMode` (`GameplayStatics.GetGameMode`)))
  (bind _output (`|GetArrayItem` (`CardCollection.Contents` (`CardGameMode.PlayedCards` _asbp_card_game_mode)) _id))
  (if (< _output 0)
    (`self.OWN-AddCardToPlayedSlot`)
    (else
      (`self.OWN-SwapSelectedHandCardWithSlot` _output _id))))

(event `OWN-SwapSelectedHandCardWithSlot`
  (params (ID :type Integer) (Location :type Integer))
  ;[1 1 1] "Swap" Hand card and Played Card Mat card
  (bind _asbp_player_state (cast `/Game/Blueprint/Online/BP_PlayerState` (`GameplayStatics.GetPlayerState` 0)))
  (`/Game/Blueprint/Online/BP_PlayerState.OWN-GetSelectedCard` _asbp_player_state)
  (bind _selectedcardinhandlocation (`/Game/Blueprint/Online/BP_PlayerState.SelectedCardInHandLocation` _asbp_player_state))
  (if (>= _selectedcardinhandlocation 0)
    (`self.SRV-Set Played Card` (`/Game/Blueprint/Online/BP_PlayerState.SelectedCardInHandID` _asbp_player_state) Location)
    (`/Game/Blueprint/Online/BP_PlayerState.OWN-RemoveHandCardAtLocation` _asbp_player_state _selectedcardinhandlocation)
    (`/Game/Blueprint/Online/BP_PlayerState.OWN-AddCardToHand` _asbp_player_state ID _selectedcardinhandlocation)))

(fn `CanDrawCard`
  (returns (bCanDraw :type Boolean))
  (return false))

(fn `UserConstructionScript`)