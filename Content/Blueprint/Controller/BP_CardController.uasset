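; Player controller for a multiplayer card game, handling each player's UI, sound cues and hand refills.
; OWN-prefixed events spawn and update waiting, countdown, heart, win and game-over widgets, and set whether the player can play.
; FillHand adds random DataTable rows to the PlayerState's hand until it reaches capacity.
; Health updates trigger the matching heart-loss effect with a defeat sound, and BeginPlay enables the mouse cursor.
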(event `OWN-UpdateHeartWidget`
  (params (Health :type Integer))
  (bind _heartswidget (`self.HeartsWidget`))
  (if (== Health 2)
    (`/Game/Blueprint/Widget/WBP_Hearts.Life 1 Lost` _heartswidget)
    ;[0.1707 0.2079 1] SFX-Defeat
    (`GameplayStatics.PlaySound2D` "/Game/Sounds/SFX/S_Defeat_Cue.S_Defeat_Cue" 1.0 1.0 0.0 null null :!label _label)
    (elif (== Health 1)
      (`/Game/Blueprint/Widget/WBP_Hearts.Life 2 Lost` _heartswidget)
      (goto _label)
      (elif (== Health 0)
        (`/Game/Blueprint/Widget/WBP_Hearts.Life 3 Lost` _heartswidget)
        (goto _label)))))

(event `OWN-Launch TimeIsUp`
  (`/Game/Blueprint/Widget/WBP_TimeIsUp.TimeIsUp` (`self.TimeIsUp`)))

(event `OWN-FillHand`
  (params (`Data Table` :type "DataTable Object Reference"))
  ;[0 0.1733 1] SFX-DrawCard
  (`GameplayStatics.PlaySound2D` "/Game/Sounds/SFX/S_Draw_Cue.S_Draw_Cue" 1.0 1.0 0.0 null null)
  (bind _asbp_player_state (cast `/Game/Blueprint/Online/BP_PlayerState` (`GameplayStatics.GetPlayerState` 0)))
  (bind _hand (`CGPlayerState.Hand` _asbp_player_state))
  (while (< (`KismetArrayLibrary.Array_Length` (`CardCollection.Contents` _hand)) (`CardCollection.MaxCapacity` _hand))
    (bind _outrownames (`DataTableFunctionLibrary.GetDataTableRowNames` `Data Table`))
    (`/Game/Blueprint/Online/BP_PlayerState.OWN-AddCardToHand` _asbp_player_state (`.OutIndex` (`KismetArrayLibrary.Array_Random` _outrownames)) 0)
    (`/Game/Blueprint/Widget/WBP_StartingTimer.StartingCountdownWBP` (`self.StartingTimer`))))

(event `self.ReceiveBeginPlay`
  (`self.SRV_ShowMouseCursor`))

(event `OWN-SpawnWinUI`
  (bind _winwidget (`self.WinWidget`))
  (bind _winwidget_2 (`self.WinWidget`))
  (bind _returnvalue (`|CreateWidget` "/Game/Blueprint/Widget/WBP_Win.WBP_Win_C" self))
  (bind _output_get (set `self.WinWidget` _returnvalue))
  (`UserWidget.AddToViewport` _output_get 0)
  (`UserWidget.PlayAnimation` _winwidget_2 (`/Game/Blueprint/Widget/WBP_Win.MenuAppears` _winwidget_2) 0.0 1 "Forward" 1.0 false)
  (`UserWidget.PlayAnimation` _winwidget (`/Game/Blueprint/Widget/WBP_Win.StarsAnim` _winwidget) 0.0 0 "Forward" 0.2 false))

(event `OWN-SpawnGameOverUI`
  (bind _gameoverwidget (`self.GameOverWidget`))
  (bind _gameoverwidget_2 (`self.GameOverWidget`))
  (bind _returnvalue (`|CreateWidget` "/Game/Blueprint/Widget/WBP_Fail.WBP_Fail_C" self))
  (bind _output_get (set `self.GameOverWidget` _returnvalue))
  (`UserWidget.AddToViewport` _output_get 0)
  (`UserWidget.PlayAnimation` _gameoverwidget_2 (`/Game/Blueprint/Widget/WBP_Fail.MenuAppears` _gameoverwidget_2) 0.0 1 "Forward" 1.0 false)
  (`UserWidget.PlayAnimation` _gameoverwidget (`/Game/Blueprint/Widget/WBP_Fail.SkullsAnim` _gameoverwidget) 0.0 0 "Forward" 0.2 false))

(event `SRV_ShowMouseCursor`
  (set `self.bShowMouseCursor` true))

(event `OWN-SpawnHostUI`
  (params (UIToSpawn :type "/Game/Blueprint/Widget/WBP_HostUI Class Reference") (MaxPlayersNeeded :type Integer) (NumberOfPlayers :type Integer))
  (bind _returnvalue (`|CreateWidget` UIToSpawn self))
  (set `TextBlock.Text` (`KismetTextLibrary.Conv_StringToText` (`KismetStringLibrary.Concat_StrStr` (`KismetStringLibrary.Concat_StrStr` (`KismetStringLibrary.Concat_StrStr` (`KismetStringLibrary.Concat_StrStr` "Waiting for players...(" (`KismetStringLibrary.Conv_IntToString` NumberOfPlayers)) "/") (`KismetStringLibrary.Conv_IntToString` MaxPlayersNeeded)) ")")) (`/Game/Blueprint/Widget/WBP_HostUI.StartingText` _returnvalue))
  (`UserWidget.AddToViewport` _returnvalue 0))

(event `OWN-RemoveWidgets`
  (`WidgetLayoutLibrary.RemoveAllWidgets`))

(event `OWN-SpawnCountdownWidget`
  (params (PlayPhaseTime :type "Float (double-precision)"))
  (bind _returnvalue (`|CreateWidget` "/Game/Blueprint/Widget/WBP_Countdown.WBP_Countdown_C" self))
  (bind _output_get (set `self.CountdownWidget` _returnvalue))
  (`/Game/Blueprint/Widget/WBP_Countdown.OWN-SetBarAllTimers` _output_get PlayPhaseTime)
  (`UserWidget.AddToViewport` _returnvalue 0)
  (`UserWidget.AddToViewport` _output_get 0))

(event `OWN-SpawnHeartUI`
  (bind _returnvalue (`|CreateWidget` "/Game/Blueprint/Widget/WBP_Hearts.WBP_Hearts_C" self))
  (bind _output_get (set `self.HeartsWidget` _returnvalue))
  (`UserWidget.AddToViewport` _output_get 0))

(event `OWN-UpdateCountdownWidget`
  (params (TimeToSet :type "Float (double-precision)"))
  (`/Game/Blueprint/Widget/WBP_Countdown.OWN-SetBarCurrentTime` (`self.CountdownWidget`) TimeToSet))

(event `OWN-SetPlayable`
  (params (CanPlay :type Boolean))
  (set `self.bCanPlay` CanPlay))

(fn `UserConstructionScript`)