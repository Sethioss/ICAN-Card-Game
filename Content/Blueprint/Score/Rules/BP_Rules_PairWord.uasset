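; BP_Rules_PairWord is a score rule that checks whether a set of cards contains a pair sharing the same placement.
; BValidateRule tallies Amplification, Body and Flavor placements from each card's CardDataComp, passing if any tally equals exactly two.
; It reads cards through a separate Index that advances only on a match, so one loop pass can consume several consecutive cards.
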(fn `bValidateRule`
  (params (Cards :type "Array of Card Object Reference (by ref)"))
  (returns (ReturnValue :type Boolean))
  (bind _placement (`CardData.Placement` (`Card.CardDataComp` (`|GetArrayItem` Cards (`self.Index`)))))
  (for _ Cards
    (`|ExecutionSequence`
      (:`then_0`
        (if (`|EnumEquality` _placement "AMPLIFICATION")
          (bind _result (`/Engine/EditorBlueprintResources/StandardMacros.IncrementInt` (`self.Amplification`))
            (:`  `
              (set `self.Amplification` _result)
              (bind _result_2 (`/Engine/EditorBlueprintResources/StandardMacros.IncrementInt` (`self.Index`))
                (:`  `
                  (set `self.Index` _result_2)))))))
      (:`then_1`
        (if (`|EnumEquality` _placement "BODY")
          (bind _result_3 (`/Engine/EditorBlueprintResources/StandardMacros.IncrementInt` (`self.Body`))
            (:`  `
              (set `self.Body` _result_3)
              (bind _result_4 (`/Engine/EditorBlueprintResources/StandardMacros.IncrementInt` (`self.Index`))
                (:`  `
                  (set `self.Index` _result_4)))))))
      (:`then_2`
        (if (`|EnumEquality` _placement "FLAVOR")
          (bind _result_5 (`/Engine/EditorBlueprintResources/StandardMacros.IncrementInt` (`self.Flavor`))
            (:`  `
              (set `self.Flavor` _result_5)
              (bind _result_6 (`/Engine/EditorBlueprintResources/StandardMacros.IncrementInt` (`self.Index`))
                (:`  `
                  (set `self.Index` _result_6)))))))))
  (if (or (== (`self.Amplification`) 2) (== (`self.Body`) 2) (== (`self.Flavor`) 2))
    (return true)
    (else
      (return false))))