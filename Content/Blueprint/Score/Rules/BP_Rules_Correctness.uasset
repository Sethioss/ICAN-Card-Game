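; Score rule Blueprint that checks whether a set of cards is placed in the correct order.
; bValidateRule walks the given cards with a running index and compares each card's CardDataComp Placement to that index.
; It fails on the first mismatch and passes when every card sits at its expected position.
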(fn `bValidateRule`
  (params (Cards :type "Array of Card Object Reference (by ref)"))
  (returns (ReturnValue :type Boolean))
  (bind _index (`self.Index`))
  (for _ Cards
    (if (!= (`CardData.Placement` (`Card.CardDataComp` (`|GetArrayItem` Cards _index))) _index)
      (return false)
      (else
        (bind _result (`/Engine/EditorBlueprintResources/StandardMacros.IncrementInt` (`self.Index`))
          (:`  `
            (set `self.Index` _result))))))
  (return true))